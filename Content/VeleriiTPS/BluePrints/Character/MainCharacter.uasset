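; Third-person player character with movement, sprint, jump, aiming via a smoothed spring-arm zoom, and health.
; Capsule overlaps track the nearby interactable and weapon for Interact, which toggles objects or swaps the attached weapon.
; Fire input or the Fire event drives the held weapon and attack montage.
; Point damage adds headshot multipliers and hit reactions, suppressing duplicate AnyDamage; death drops the weapon, ragdolls with an impulse, then destroys the actor.
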(event OnComponentBeginOverlap(CapsuleComponent)
  (params (OverlappedComponent :type Primitive%20Component%20Object%20Reference) (OtherActor :type Actor%20Object%20Reference) (OtherComp :type Primitive%20Component%20Object%20Reference) (OtherBodyIndex :type Integer) (bFromSweep :type Boolean) (SweepResult :type Hit%20Result%20Structure%20%28by%20ref%29))
  (Utilities|FlowControl|Sequence
    (:then_0
      ;[1 1 1] Cast это функция которая делает попытку привести один тип данных к другому типу данных. При этом на вход подается ссылка а на объект. А на выходе мы получаем ссылку на дочерний объект.
      ;;[0 0.01767 0.25] Cast - уточнение типа данных
      (bind _asbase_interact (Utilities|Casting|CastToBaseInteract OtherActor))
      (Variables|Default|SetInteractReference _asbase_interact))
    (:then_1
      (bind _asbase_weapon (Utilities|Casting|CastToBaseWeapon OtherActor))
      (Variables|Default|SetWeaponRefInteract _asbase_weapon))))

(event OnComponentEndOverlap(CapsuleComponent)
  (params (OverlappedComponent :type Primitive%20Component%20Object%20Reference) (OtherActor :type Actor%20Object%20Reference) (OtherComp :type Primitive%20Component%20Object%20Reference) (OtherBodyIndex :type Integer))
  (Utilities|FlowControl|Sequence
    (:then_0
      (bind _asbase_interact (Utilities|Casting|CastToBaseInteract OtherActor))
      (if (== _asbase_interact (Variables|Default|GetInteractReference))
        (Variables|Default|SetInteractReference 0)))
    (:then_1
      (bind _asbase_weapon (Utilities|Casting|CastToBaseWeapon OtherActor))
      (if (== _asbase_weapon (Variables|Default|GetWeaponRefInteract))
        (Variables|Default|SetWeaponRefInteract 0)))))

(event Custom|InitCharacter
  (Variables|Default|SetHP_Current (Variables|Default|GetHP_Max%28const%29)))

(event Custom|DeathHandling
  (Utilities|FlowControl|DoOnce false
    (:Completed
      (Variables|Default|SetIAmAlive false)
      (Physics|SetSimulatePhysics (Variables|Character|GetMesh) true)
      (Physics|AddImpulse (Variables|Character|GetMesh) (Variables|Default|GetHitDirection) (Variables|Default|GetHitBone) true)
      (Pawn|Components|CharacterMovement|DisableMovement (Variables|Character|GetCharacterMovement))
      (CallFunction|DropItem)
      (Utilities|FlowControl|Delay 5.0)
      (Actor|DestroyActor))))

(event Custom|Fire
  (params (Activate :type Boolean))
  (bind _weaponrefactive (Variables|Default|GetWeaponRefActive))
  (bind _weaponrefactive_2 (Variables|Default|GetWeaponRefActive))
  ;[1 1 1] Входные данные
  (if Activate
    (if (Utilities|IsValid _weaponrefactive_2)
      (Default|FireBaseWeapon _weaponrefactive_2 true)
      (Animation|Montage|PlayMontage (Variables|Character|GetMesh) (Variables|Default|GetAttackMontage)))
    (elif (Utilities|IsValid _weaponrefactive)
      (Default|FireBaseWeapon _weaponrefactive false))))

(event EventTick
  (params (DeltaSeconds :type Float%20%28single-precision%29))
  ;[1 0 0] Event tick
  (Variables|/Script/Engine.SpringArmComponent|SetTargetArmLength (Variables|Default|GetSpringArm) (Math|Float|Lerp (Variables|/Script/Engine.SpringArmComponent|GetTargetArmLength (Variables|Default|GetSpringArm)) (Variables|Default|GetTargetSpringArmLenght) 0.1)))

(event EventBeginPlay
  (CallFunction|InitCharacter))

(event Game|Damage|EventAnyDamage
  (params (Damage :type Float%20%28single-precision%29) (DamageType :type Damage%20Type%20Object%20Reference) (InstigatedBy :type Controller%20Object%20Reference) (DamageCauser :type Actor%20Object%20Reference))
  (if (not (Variables|Default|GetHasPointDamage))
    (bind _characterdead (CallFunction|ApplyDamage Damage))
    (if _characterdead
      (CallFunction|DeathHandling))))

(event Game|Damage|EventPointDamage
  (params (Damage :type Float%20%28single-precision%29) (DamageType :type Damage%20Type%20Object%20Reference) (HitLocation :type Vector :default "0, 0, 0") (HitNormal :type Vector :default "0, 0, 0") (HitComponent :type Primitive%20Component%20Object%20Reference) (BoneName :type Name :default "None") (ShotFromDirection :type Vector :default "0, 0, 0") (InstigatedBy :type Controller%20Object%20Reference) (DamageCauser :type Actor%20Object%20Reference) (HitInfo :type Hit%20Result%20Structure%20%28by%20ref%29))
  (Variables|Default|SetHitDirection ShotFromDirection)
  (Variables|Default|SetHitBone (.HitBoneName (Collision|BreakHitResult HitInfo)))
  (Variables|Default|SetDamage Damage)
  (Variables|Default|SetHasPointDamage true)
  (Utilities|FlowControl|Sequence
    (:then_0
      (if (Utilities|Name|Equal(Name) (Variables|Default|GetHitBone) "head")
        (bind _characterdead (CallFunction|ApplyDamage (* (Variables|Default|GetDamage) (Variables|Default|GetCriticalMul))))
        (else
          (bind _characterdead_2 (CallFunction|ApplyDamage (Variables|Default|GetDamage)))))
      (if (or _characterdead _characterdead_2)
        (CallFunction|DeathHandling)
        (Utilities|FlowControl|Delay 0.2)
        (Variables|Default|SetHasPointDamage false)))
    (:then_1
      (Animation|Montage|PlayMontage (Variables|Character|GetMesh) "/Game/AnimStarterPack/Hit_React_4_Montage.Hit_React_4_Montage"))))

(event Input|ActionEvents|InputActionInteract
  (params (Key :type Key%20Structure :default "None"))
  (bind _interactreference (Variables|Default|GetInteractReference))
  ;[1 1 1] Входные данные
  (:Pressed
    (Utilities|FlowControl|Sequence
      (:then_0
        ;[1 1 1] Проверка валидности. То есть мы проверяем что в ссылке что-либо записано
        (if (Utilities|IsValid (Variables|Default|GetInteractReference))
          (Default|ActivateInteract _interactreference (not (Variables|/Game/VeleriiTPS/BluePrints/Interract/BaseInteract.BaseInteract_C|GetIsActive _interactreference)))))
      (:then_1
        (if (Utilities|IsValid (Variables|Default|GetWeaponRefInteract))
          (if (Utilities|IsValid (Variables|Default|GetWeaponRefActive))
            (CallFunction|DropItem)
            (CallFunction|TakeItem)
            (else
              (CallFunction|TakeItem))))))))

(event Input|ActionEvents|InputActionSprint
  (params (Key :type Key%20Structure :default "None"))
  ;[1 1 1] Входные данные
  (:Pressed
    (Variables|/Script/Engine.CharacterMovementComponent|SetMaxWalkSpeed (Variables|Character|GetCharacterMovement) 9e+02))
  (:Released
    (Variables|/Script/Engine.CharacterMovementComponent|SetMaxWalkSpeed (Variables|Character|GetCharacterMovement) 4.5e+02)))

(event Input|ActionEvents|InputActionFire
  (params (Key :type Key%20Structure :default "None"))
  (bind _weaponrefactive (Variables|Default|GetWeaponRefActive))
  (bind _weaponrefactive_2 (Variables|Default|GetWeaponRefActive))
  ;[1 1 1] Входные данные
  (:Pressed
    (if (Utilities|IsValid _weaponrefactive_2)
      (Default|FireBaseWeapon _weaponrefactive_2 true)
      (Animation|Montage|PlayMontage (Variables|Character|GetMesh) (Variables|Default|GetAttackMontage))))
  (:Released
    (if (Utilities|IsValid _weaponrefactive)
      (Default|FireBaseWeapon _weaponrefactive false))))

(event Input|ActionEvents|InputActionDropItem
  (params (Key :type Key%20Structure :default "None"))
  ;[1 1 1] Входные данные
  (:Pressed
    (CallFunction|DropItem)))

(event Input|ActionEvents|InputActionAim
  (params (Key :type Key%20Structure :default "None"))
  ;[1 1 1] Входные данные
  (:Pressed
    (Variables|Default|SetTargetSpringArmLenght 5e+01)
    (Variables|Default|SetOnAim true))
  (:Released
    (Variables|Default|SetTargetSpringArmLenght 3e+02)
    (Variables|Default|SetOnAim false)))

(event Input|ActionEvents|InputActionJump
  (params (Key :type Key%20Structure :default "None"))
  ;[1 1 1] Входные данные
  (:Pressed
    (Character|Jump)))

(event Input|AxisEvents|InputAxisMoveForward
  (params (AxisValue :type Float%20%28single-precision%29))
  ;[1 1 1] Входные данные
  (Pawn|Input|AddMovementInput (Transformation|GetActorForwardVector) AxisValue false))

(event Input|AxisEvents|InputAxisMoveRight
  (params (AxisValue :type Float%20%28single-precision%29))
  ;[1 1 1] Входные данные
  (Pawn|Input|AddMovementInput (Transformation|GetActorRightVector) AxisValue false))

(event Input|AxisEvents|InputAxisLookUp
  (params (AxisValue :type Float%20%28single-precision%29))
  ;[1 1 1] Входные данные
  (Pawn|Input|AddControllerPitchInput AxisValue))

(event Input|AxisEvents|InputAxisTurn
  (params (AxisValue :type Float%20%28single-precision%29))
  ;[1 1 1] Входные данные
  (Pawn|Input|AddControllerYawInput AxisValue))

(fn ConstructionScript)

(fn DropItem
  (if (Utilities|IsValid (Variables|Default|GetWeaponRefActive))
    (Transformation|DetachFromActor (Variables|Default|GetWeaponRefActive) "KeepWorld" "KeepWorld" "KeepWorld")
    (Physics|SetSimulatePhysics (Variables|/Game/VeleriiTPS/BluePrints/Weapon/BaseWeapon.BaseWeapon_C|GetStaticMesh (Variables|Default|GetWeaponRefActive)) true)
    (Variables|Default|SetWeaponRefActive 0)))

(fn TakeItem
  (Variables|Default|SetWeaponRefActive (Variables|Default|GetWeaponRefInteract))
  (Transformation|AttachComponentToComponent (Variables|Default|GetWeaponRefActive) (Variables|Default|GetWeaponPlace) "None" "SnapToTarget" "SnapToTarget" "KeepWorld" true)
  (Physics|SetSimulatePhysics (Variables|/Game/VeleriiTPS/BluePrints/Weapon/BaseWeapon.BaseWeapon_C|GetStaticMesh (Variables|Default|GetWeaponRefInteract)) false)
  (Variables|Default|SetWeaponRefInteract 0))

(fn ApplyDamage
  (params (Damage :type Float%20%28single-precision%29))
  (Variables|Default|SetHP_Current (Math|Float|Clamp(Float) (- (Variables|Default|GetHP_Current) Damage) 0.0 (Variables|Default|GetHP_Max%28const%29)))
  (return (== (Variables|Default|GetHP_Current) 0.0)))
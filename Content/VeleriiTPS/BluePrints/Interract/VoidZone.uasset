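; VoidZone is a damage area actor that continuously hurts actors inside its Box collision component.
; Box overlap events add entering actors to a Targets array and remove them when they leave, with no filtering by actor type.
; Tick applies DamagePerSec scaled by delta time to every tracked actor, so damage over time stays independent of frame rate.
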(event OnComponentBeginOverlap(Box)
  (params (OverlappedComponent :type Primitive%20Component%20Object%20Reference) (OtherActor :type Actor%20Object%20Reference) (OtherComp :type Primitive%20Component%20Object%20Reference) (OtherBodyIndex :type Integer) (bFromSweep :type Boolean) (SweepResult :type Hit%20Result%20Structure%20%28by%20ref%29))
  ;[1 1 1] Добавление предмета в массив
  (Utilities|Array|Add (Variables|Default|GetTargets) OtherActor))

(event OnComponentEndOverlap(Box)
  (params (OverlappedComponent :type Primitive%20Component%20Object%20Reference) (OtherActor :type Actor%20Object%20Reference) (OtherComp :type Primitive%20Component%20Object%20Reference) (OtherBodyIndex :type Integer))
  ;[1 1 1] удаление предмета из массива
  (Utilities|Array|RemoveItem (Variables|Default|GetTargets) OtherActor))

(event EventTick
  (params (DeltaSeconds :type Float%20%28single-precision%29))
  (if (> (Utilities|Array|Length (Variables|Default|GetTargets)) 0)
    ;[1 1 1] For пробегает по всем элементам массива
    (for _array_element (Variables|Default|GetTargets)
      (Game|Damage|ApplyDamage _array_element (* (Variables|Default|GetDamagePerSec) DeltaSeconds) 0 0))))

(fn ConstructionScript)
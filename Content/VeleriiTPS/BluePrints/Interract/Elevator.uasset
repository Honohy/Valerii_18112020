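; Interactable elevator that carries a static mesh along a spline path when activated or deactivated.
; The ActivateInteract event calls the parent logic, then passes its Activate flag to ElevatorStart.
; ElevatorStart plays or reverses the ElevatorMoving timeline, whose Scale track samples the spline by time to set the mesh's world location without sweep.
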(event Custom|ElevatorStart
  (params (StartStop :type Boolean))
  (bind _output_get (Variables|Default|SetStart/Stop StartStop))
  (if _output_get
    (bind _scale (Timeline|ElevatorMoving Play)
      (:Update
        (Transformation|SetWorldLocation (Variables|Default|GetStaticMesh) (Spline|GetLocationatTime (Variables|Default|GetSpline) _scale "World" false) false false)))
    (else
      (Timeline|ElevatorMoving Reverse))))

(event EventActivateInteract
  (params (Activate :type Boolean))
  (|CallParentFunction Activate)
  (CallFunction|ElevatorStart Activate))

(fn ConstructionScript
  (|CallParentFunction))
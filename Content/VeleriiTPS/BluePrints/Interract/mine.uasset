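; Proximity mine actor that explodes when another actor enters its trigger sphere.
; On sphere overlap it applies point damage to the overlapping actor, with a scaled hit direction pointing away from the mine and a fabricated hit on the spine bone.
; It then spawns an explosion particle effect and sound at its location and destroys itself.
; Only the triggering actor takes damage; there is no radial falloff or actor filtering.
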(event OnComponentBeginOverlap(Sphere)
  (params (OverlappedComponent :type Primitive%20Component%20Object%20Reference) (OtherActor :type Actor%20Object%20Reference) (OtherComp :type Primitive%20Component%20Object%20Reference) (OtherBodyIndex :type Integer) (bFromSweep :type Boolean) (SweepResult :type Hit%20Result%20Structure%20%28by%20ref%29))
  (Variables|Default|SetHitDirection (* (Math|Vector|Normalize (- (Transformation|GetActorLocation OtherActor) (Transformation|GetActorLocation))) 5000))
  (Game|Damage|ApplyPointDamage OtherActor (Variables|Default|GetDamage) (Variables|Default|GetHitDirection) (Collision|MakeHitResult false false 0.0 0.0 "0, 0, 0" "0.000000, 0, 0" "0,0,1" "0,0,1" 0 0 0 "spine_01"))
  (Effects|SpawnEmitteratLocation "/Game/Download/StarterContent/Particles/P_Explosion.P_Explosion" (Transformation|GetActorLocation) "0, 0, 0" "5.000000,5.000000,5.000000")
  (Audio|SpawnSoundatLocation "/Game/Download/StarterContent/Audio/Explosion_Cue.Explosion_Cue" (Transformation|GetActorLocation) "0, 0, 0" 1.0 1.0 0.0 0 0)
  (Actor|DestroyActor))

(event EventBeginPlay)

(event Collision|EventActorBeginOverlap
  (params (OtherActor :type Actor%20Object%20Reference)))

(event EventTick
  (params (DeltaSeconds :type Float%20%28single-precision%29)))

(fn ConstructionScript)